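; Pinball player controller that routes input to flippers and plunger, respawns the ball on death and tracks score on a chalkboard.
; On BeginPlay it caches left/right flippers, plunger, spawner and scoreboard, then spawns a ball.
; DoQuicktimeEvent freezes the ball and repurposes the three controls as answers to random timed prompts.
; It repeats while keys remain, stops on failure, then reports the result to the calling entity and unfreezes.
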(event Custom|BallDeath
  (params (Ball :type Ball%20Object%20Reference))
  (Actor|DestroyActor Ball)
  (bind _ball (CallFunction|SpawnBall))
  (Variables|Default|SetBall _ball))

(event Custom|DoQuicktimeEvent
  (params (CallingEntity :type Quicktime%20Entity%20Base%20BP%20Object%20Reference))
  (Variables|Quicktime|SetInQuicktime true)
  (Default|Freeze (Variables|Default|GetBall))
  (bind _returnvalue (Game|ConstructObjectfromClass "/Game/Pinball/BP/Widgets/QuicktimeWidget.QuicktimeWidget_C" self))
  (bind _output_get (Variables|Quicktime|SetQuicktimeWidget _returnvalue))
  (UserInterface|Viewport|AddtoViewport _output_get 0)
  (Variables|Quicktime|SetQuicktimeSuccess false :!label _label)
  (bind _output_get_2 (Variables|Quicktime|SetNextQuicktimeKey (Math|Random|RandomInteger 3)))
  (Default|SelectButton _output_get (+ _output_get_2 1))
  (Utilities|FlowControl|Delay 4.0)
  (if (Variables|Quicktime|GetQuicktimeSuccess)
    (bind _result (Math|Integer|DecrementInt (Variables|Quicktime|GetNumQuicktimeKeys))
      (:%20%20
        (if (> _result 0)
          (Utilities|FlowControl|Delay 0.5)
          (goto _label)
          (else
            _))))
    (else
      (Default|AnswerHighlight (Variables|Quicktime|GetQuicktimeWidget) (Variables|Quicktime|GetQuicktimeSuccess))))
  (Utilities|FlowControl|Delay 1.5)
  (Default|RecieveQuicktimeResults CallingEntity (Variables|Quicktime|GetQuicktimeSuccess))
  (Widget|RemovefromParent (Variables|Quicktime|GetQuicktimeWidget))
  (Variables|Quicktime|SetInQuicktime false)
  (Default|Unfreeze (Variables|Default|GetBall)))

(event EventBeginPlay
  (Utilities|FlowControl|Sequence
    (:then_0
      (bind _outactors (Actor|GetAllActorsOfClass "/Game/Pinball/BP/Actors/Flippers/FlipperBase_AbstractBP.FlipperBase_AbstractBP_C"))
      (for _array_element _outactors
        (bind _asflipper_left_bp (Utilities|Casting|CastToFlipperLeft_BP _array_element)
          (:then
            (Utilities|Array|AddUnique (Variables|Default|GetLeftFlippers) _asflipper_left_bp))
          (:CastFailed
            (bind _asflipper_right_bp (Utilities|Casting|CastToFlipperRight_BP _array_element))
            (Utilities|Array|AddUnique (Variables|Default|GetRightFlippers) _asflipper_right_bp)))))
    (:then_1
      (bind _returnvalue (Actor|GetActorOfClass "/Game/Pinball/BP/Actors/Plunger/Plunger_BP.Plunger_BP_C"))
      (Variables|Default|SetPlunger _returnvalue))
    (:then_2
      (bind _returnvalue_2 (Actor|GetActorOfClass "/Game/Pinball/BP/Actors/Ball/BallSpawn_BP.BallSpawn_BP_C"))
      (Variables|Default|SetBall%20Spawn _returnvalue_2)
      (CallFunction|SpawnBall))
    (:then_3
      (bind _returnvalue_3 (Actor|GetActorOfClass "/Game/Pinball/BP/Actors/UI_ELements/ScoreChalkboard.ScoreChalkboard_C"))
      (Variables|Default|SetScore%20Chalkboard _returnvalue_3))))

(event Input|ActionEvents|InputActionFlipperLeft
  (params (Key :type Key%20Structure :default "None"))
  (bind _leftflippers (Variables|Default|GetLeftFlippers))
  (bind _inquicktime (Variables|Quicktime|GetInQuicktime))
  (:Pressed
    (if _inquicktime
      (bind _output_get (Variables|Quicktime|SetQuicktimeSuccess (== (Variables|Quicktime|GetNextQuicktimeKey) 0)))
      (Default|AnswerHighlight (Variables|Quicktime|GetQuicktimeWidget) _output_get)
      (else
        (for _array_element _leftflippers
          (Default|ActivateFlipper _array_element)))))
  (:Released
    (if (not _inquicktime)
      (for _array_element_2 _leftflippers
        (Default|RetractFlipper _array_element_2)))))

(event Input|ActionEvents|InputActionFlipperRight
  (params (Key :type Key%20Structure :default "None"))
  (bind _rightflippers (Variables|Default|GetRightFlippers))
  (bind _inquicktime (Variables|Quicktime|GetInQuicktime))
  (:Pressed
    (if _inquicktime
      (bind _output_get (Variables|Quicktime|SetQuicktimeSuccess (== (Variables|Quicktime|GetNextQuicktimeKey) 2)))
      (Default|AnswerHighlight (Variables|Quicktime|GetQuicktimeWidget) _output_get)
      (else
        (for _array_element _rightflippers
          (Default|ActivateFlipper _array_element)))))
  (:Released
    (if (not _inquicktime)
      (for _array_element_2 _rightflippers
        (Default|RetractFlipper _array_element_2)))))

(event Input|ActionEvents|InputActionShootBall
  (params (Key :type Key%20Structure :default "None"))
  (bind _inquicktime (Variables|Quicktime|GetInQuicktime))
  (bind _plunger (Variables|Default|GetPlunger))
  (:Pressed
    (if _inquicktime
      (bind _output_get (Variables|Quicktime|SetQuicktimeSuccess (== (Variables|Quicktime|GetNextQuicktimeKey) 1)))
      (Default|AnswerHighlight (Variables|Quicktime|GetQuicktimeWidget) _output_get)
      (else
        (Default|PlungerRetract _plunger))))
  (:Released
    (if (not _inquicktime)
      (Default|PlungerRelease _plunger))))

(fn ConstructionScript)

(fn SpawnBall
  (bind _ball (Default|SpawnBall (Variables|Default|GetBall%20Spawn)))
  (bind _output_get (Variables|Default|SetBall _ball))
  (return _output_get))

(fn UpdateScore
  (params (ScoreToAdd :type Integer))
  (bind _output_get (Variables|Default|SetScore (+ (stale _output_get) ScoreToAdd)))
  (Default|UpdateScoreRender (Variables|Default|GetScore%20Chalkboard) (Utilities|Text|ToText(Integer) _output_get)))