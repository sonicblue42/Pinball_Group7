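; DeathZone_BP is a pinball drain volume that reports balls entering it to the player controller.
; At BeginPlay it caches the PinballController_BP, and on actor overlap it passes any Ball to that controller's BallDeath, with a debug print on every overlap.
; The construction script scales the DeathZoneBoundary component by the DeathZoneSize variable.
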(event EventBeginPlay
  (bind _aspinball_controller_bp (Utilities|Casting|CastToPinballController_BP (Game|GetPlayerController 0)))
  (Variables|Default|SetController _aspinball_controller_bp))

(event Collision|EventActorBeginOverlap
  (params (OtherActor :type Actor%20Object%20Reference))
  (Development|PrintString "OVERLAP")
  (bind _asball (Utilities|Casting|CastToBall OtherActor))
  (Default|BallDeath (Variables|Default|GetController) _asball))

(event EventTick
  (params (DeltaSeconds :type Float%20%28single-precision%29)))

(fn ConstructionScript
  (Transformation|SetWorldScale3D (Variables|Default|GetDeathZoneBoundary) (Variables|Default|GetDeathZoneSize)))