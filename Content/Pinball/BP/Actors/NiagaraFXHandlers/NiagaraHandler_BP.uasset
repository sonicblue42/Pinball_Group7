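; Self-destroying actor that plays a one-shot Niagara effect in the pinball game.
; On BeginPlay it assigns the given system to its Niagara component, passes the target as the TargetLocation parameter and activates it.
; If the target is non-zero, the actor also rotates to face it.
; It destroys itself when the system finishes.
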(event OnSystemFinished(Niagara)
  (params (PSystem :type Niagara%20Component%20Object%20Reference))
  (Actor|DestroyActor))

(event EventBeginPlay
  (bind _target (Variables|Default|GetTarget))
  (Class|NiagaraComponent|SetAsset (Variables|Default|GetNiagara) (Variables|Default|GetNiagara%20System))
  (Effects|Components|ParticleSystem|SetVectorParameter (Variables|Default|GetNiagara) "TargetLocation" _target)
  (Components|Activation|Activate (Variables|Default|GetNiagara) true)
  (if (Math|Vector|NotEqual(Vector) _target "0, 0, 0" 0.0001)
    (Transformation|SetActorRotation (Math|Rotator|FindLookatRotation (Transformation|GetActorLocation) _target))))

(fn ConstructionScript)