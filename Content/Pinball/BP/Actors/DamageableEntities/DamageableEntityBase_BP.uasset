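; Base actor for damageable entities in the pinball game, providing health, hit handling and death.
; Hit subtracts damage while CanBeHit is set, logs the result, and reports whether it hit and killed.
; A surviving hit starts invincibility frames that block further hits for IFramesDuration.
; At zero health, Die spawns a NiagaraHandler_BP radial burst at the actor's transform and destroys it.
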(event Custom|Do%20IFrames
  (Variables|Default|SetCanBeHit false)
  (Utilities|FlowControl|Delay (Variables|Default|GetIFramesDuration))
  (Variables|Default|SetCanBeHit true))

(event EventBeginPlay)

(fn ConstructionScript)

(fn Hit
  (params (Damage :type Integer))
  (if (Variables|Default|GetCanBeHit)
    (bind _output_get (Variables|Default|SetHealth (- (Variables|Default|GetHealth) Damage)))
    (Development|PrintString (Utilities|String|Append "Damageable entity hit for " (Utilities|String|ToString(Integer) Damage) " damage, health is now " (Utilities|String|ToString(Integer) _output_get)))
    (if (<= _output_get 0)
      (CallFunction|Die)
      (return true true)
      (else
        (CallFunction|DoIFrames)
        (return true false)))
    (else
      (return false false))))

(fn Die
  (Game|SpawnActorfromClass "/Game/Pinball/BP/Actors/NiagaraFXHandlers/NiagaraHandler_BP.NiagaraHandler_BP_C" (Transformation|GetActorTransform) "Undefined" 0 "/Niagara/DefaultAssets/Templates/Systems/RadialBurst.RadialBurst" "0.000000,0.000000,0.000000" 0)
  (Actor|DestroyActor))