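; Base Blueprint for pinball damageable entities that are defeated through a quicktime event instead of by damage.
; A hit asks the player controller to start a quicktime event for this entity and add a star, then calls the parent hit with zero damage and reports no death.
; The entity dies only when the quicktime results come back successful.
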(event Custom|RecieveQuicktimeResults
  (params (Success :type Boolean))
  (if Success
    (CallFunction|Die)))

(fn ConstructionScript
  (|CallParentFunction))

(fn Hit
  (params (Damage :type Integer) (Other :type Actor%20Object%20Reference))
  (Default|DoQuicktimeEvent (Variables|Default|GetPlayerController) self)
  (Default|AddStar (Variables|Default|GetPlayerController))
  (|CallParentFunction 0 Other)
  (return true false))