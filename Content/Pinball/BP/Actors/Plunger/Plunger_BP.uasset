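; Pinball plunger actor that retracts and releases through its PlungerRetract and PlungerRelease events.
; A retract timeline scales the spring and records the current value until release interrupts it.
; A release timeline then blends from that value back to full scale and resets the state flags when finished.
; SetPlungerScale stretches the spring on Z and moves the plunger top along Y with sweep enabled.
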(event Custom|PlungerRetract
  (if (not (Variables|Default|GetIsRetracted))
    (Variables|Default|SetIsRetracted true)
    (bind _plungerretractmod (Timeline|PlungerRetractTimeline PlayFromStart)
      (:Update
        (if (Variables|Default|GetDoRelease)
          (Timeline|PlungerRetractTimeline Stop)
          (else
            (CallFunction|SetPlungerScale _plungerretractmod)
            (Variables|Default|SetPlungerRetractValue _plungerretractmod)))))))

(event Custom|PlungerRelease
  (bind _plungerretractvalue (Variables|Default|GetPlungerRetractValue))
  (if (Variables|Default|GetIsRetracted)
    (Variables|Default|SetDoRelease true)
    (bind _releasemod (Timeline|PlungerReleaseTimeline PlayFromStart)
      (:Update
        (CallFunction|SetPlungerScale (+ _plungerretractvalue (* (- 1.0 _plungerretractvalue) _releasemod))))
      (:Finished
        (Variables|Default|SetIsRetracted false)
        (Variables|Default|SetDoRelease false)))))

(fn ConstructionScript)

(fn SetPlungerScale
  (params (PlungerScale :type Float%20%28single-precision%29))
  (Transformation|SetRelativeScale3D (Variables|Default|GetSpring) (Math|Vector|MakeVector 1.0 1.0 PlungerScale))
  (Transformation|SetRelativeLocation (Variables|Default|GetPlungerTop) (Math|Vector|MakeVector 0.0 (* -5e+02 PlungerScale) 0.0) true false))