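; Abstract base actor for pinball flippers that swings a Pivot component out and back through activate and retract events.
; Separate extend and retract timelines scale FlipperTurnDegrees and add it to the resting yaw captured on activation.
; State flags block re-activation until retraction finishes and defer an early release until the extend stroke completes, so every flip travels fully out.
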(event Custom|ActivateFlipper
  (Variables|Default|SetFlipperButtonHeld true)
  (if (Variables|Default|GetCanActivate)
    (Variables|Default|SetCanActivate false)
    (Variables|Default|SetDefaultRotation (Variables|/Script/Engine.SceneComponent|GetRelativeRotation (Variables|Default|GetPivot)))
    (bind _flipperextendtrack (Timeline|FlipperExtendTimeline PlayFromStart)
      (:Update
        (Transformation|SetRelativeRotation (Variables|Default|GetPivot) (Math|Rotator|MakeRotator 0.0 0.0 (+ (* (Variables|Default|GetFlipperTurnDegrees) _flipperextendtrack) (.Yaw (Math|Rotator|BreakRotator (Variables|Default|GetDefaultRotation))))) false false))
      (:Finished
        (Variables|Default|SetFlipperOut true)
        (if (not (Variables|Default|GetFlipperButtonHeld))
          (CallFunction|RetractFlipper))))))

(event Custom|RetractFlipper
  (Variables|Default|SetFlipperButtonHeld false)
  (if (Variables|Default|GetFlipperOut)
    (Variables|Default|SetFlipperOut false)
    (bind _flipperretracttrack (Timeline|FlipperRetractTimeline PlayFromStart)
      (:Update
        (Transformation|SetRelativeRotation (Variables|Default|GetPivot) (Math|Rotator|MakeRotator 0.0 0.0 (+ (* (Variables|Default|GetFlipperTurnDegrees) _flipperretracttrack) (.Yaw (Math|Rotator|BreakRotator (Variables|Default|GetDefaultRotation))))) false false))
      (:Finished
        (Variables|Default|SetCanActivate true)))))

(event EventBeginPlay)

(event Collision|EventActorBeginOverlap
  (params (OtherActor :type Actor%20Object%20Reference)))

(event EventTick
  (params (DeltaSeconds :type Float%20%28single-precision%29)))

(fn ConstructionScript
  (Variables|Default|SetDefaultRotation (Transformation|GetActorRotation)))